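; BP_HealthPotion is a holdable pickup item meant to restore health when used.
; Overlapping its sphere asks the custom third-person character to pick it up, and Pickup attaches the potion to the hand_r socket of the given mesh.
; Drop detaches it and turns on physics and collision for the bottle body.
; PrimaryAction only prints a +10 health message, clears the character's held item and destroys the potion, without changing health.
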(event `self.Sphere.OnComponentBeginOverlap`
  (params (OverlappedComponent :type "PrimitiveComponent Object Reference") (OtherActor :type "Actor Object Reference") (OtherComp :type "PrimitiveComponent Object Reference") (OtherBodyIndex :type Integer) (bFromSweep :type Boolean) (SweepResult :type "HitResult Structure (by ref)"))
  (bind _asbp_third_person_character_custom (cast `/Game/BluePrints/BP_ThirdPersonCharacter_Custom` OtherActor))
  (`/Game/BluePrints/BP_ThirdPersonCharacter_Custom.TryToPickUp` _asbp_third_person_character_custom self))

(event `/Game/BluePrints/BPI_Item.Pickup`
  (params (`Parent Mesh` :type "SkeletalMeshComponent Object Reference"))
  (`SceneComponent.K2_AttachToComponent` (`self.DefaultSceneRoot`) `Parent Mesh` "hand_r" "SnapToTarget" "KeepRelative" "KeepRelative" true))

(event `/Game/BluePrints/BPI_Item.Drop`
  (`SceneComponent.K2_DetachFromComponent` (`self.DefaultSceneRoot`) "KeepRelative" "KeepRelative" "KeepRelative" true) ; Don't follow hand
  (`PrimitiveComponent.SetSimulatePhysics` (`self.Bottom of Body`) true)
  (`PrimitiveComponent.SetCollisionEnabled` (`self.Bottom of Body`) "QueryAndPhysics") ; Collide with ground pretty please
)

(event `/Game/BluePrints/BPI_Item.Primary Action`
  (params (ref_ThirdPersonCharCustom :type "/Game/BluePrints/BP_ThirdPersonCharacter_Custom Object Reference"))
  (`KismetSystemLibrary.PrintString` "+10 health")
  (set `/Game/BluePrints/BP_ThirdPersonCharacter_Custom.Held Item` null ref_ThirdPersonCharCustom)
  (`self.K2_DestroyActor`))

(fn `UserConstructionScript`)