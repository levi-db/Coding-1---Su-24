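; BP_Key is a collectible key pickup that the player gathers by walking into it.
; When its BoxCollision is overlapped by BP_ThirdPersonCharacter_Custom, it increments that character's KeyCount and destroys itself.
; Debug strings print on spawn, on pickup with the new key total, and when the cast fails for other overlapping actors.
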(event `self.ReceiveBeginPlay`
  (`KismetSystemLibrary.PrintString` "This Key exists " true true (struct :`R` 0.884487 :`G` 0.123094 :`B` 1.0 :`A` 1.0) 5.0))

(event `self.Box Collision.OnComponentBeginOverlap`
  (params (OverlappedComponent :type "PrimitiveComponent Object Reference") (OtherActor :type "Actor Object Reference") (OtherComp :type "PrimitiveComponent Object Reference") (OtherBodyIndex :type Integer) (bFromSweep :type Boolean) (SweepResult :type "HitResult Structure (by ref)"))
  (bind _asbp_third_person_character_custom (cast `/Game/BluePrints/BP_ThirdPersonCharacter_Custom` OtherActor)
    (:`then`
      (`KismetSystemLibrary.PrintString` "Key has been Overlapped by Player" true true (struct :`G` 0.66 :`B` 1.0 :`A` 1.0) 5.0)
      (bind _key_count (`/Game/BluePrints/BP_ThirdPersonCharacter_Custom.Key Count` _asbp_third_person_character_custom))
      (set `/Game/BluePrints/BP_ThirdPersonCharacter_Custom.Key Count` (+ _key_count 1) _asbp_third_person_character_custom)
      (`KismetSystemLibrary.PrintString` (`KismetStringLibrary.Concat_StrStr` "The Player has " (`KismetStringLibrary.Conv_IntToString` _key_count) " key(s).") true true (struct :`G` 0.66 :`B` 1.0 :`A` 1.0) 5.0)
      (`self.K2_DestroyActor`))
    (:`CastFailed`
      (`KismetSystemLibrary.PrintString` "Key Player Cast failed" true true (struct :`R` 1.0 :`B` 0.047826 :`A` 1.0) 5.0))))

(fn `UserConstructionScript`)