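; BP_FallingPlatform is a platform that falls shortly after the player steps into its trigger box, then returns to its start.
; Activate, Drop and Reset run in sequence with delays, and a Ready flag blocks retriggering until the cycle ends.
; Drop enables physics on the cube; Reset disables it and a timeline lerps the cube back to its saved starting transform.
; Each state swaps the cube's material and most print a debug message.
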(event `self.ReceiveBeginPlay`
  (set `self.Starting Transform` (`SceneComponent.K2_GetComponentToWorld` (`self.Cube`))))

(event `self.Box.OnComponentBeginOverlap`
  (params (OverlappedComponent :type "PrimitiveComponent Object Reference") (OtherActor :type "Actor Object Reference") (OtherComp :type "PrimitiveComponent Object Reference") (OtherBodyIndex :type Integer) (bFromSweep :type Boolean) (SweepResult :type "HitResult Structure (by ref)"))
  (cast `/Game/BluePrints/BP_ThirdPersonCharacter_Custom` OtherActor) ; Was it the player?
  (`self.Activate`))

(event `Activate`
  ;[1 0.5915 0.808] Platform Activates
  (if (`self.Ready`)
    (`KismetSystemLibrary.PrintString` "One second left!" true true (struct :`R` 0.501961 :`G` 0.478431 :`B` 1.0 :`A` 1.0))
    (set `self.Ready` false)
    (`PrimitiveComponent.SetMaterial` (`self.Cube`) 0 "/Game/Materials/MI_PlatformActivated.MI_PlatformActivated")
    (`KismetSystemLibrary.Delay` 1.0)
    (`self.Drop`)))

(event `Drop`
  ;[1 0.5897 0.6097] Platform Drops
  (`KismetSystemLibrary.PrintString` "Dropping!" true true (struct :`R` 0.501961 :`G` 0.478431 :`B` 1.0 :`A` 1.0))
  (`PrimitiveComponent.SetSimulatePhysics` (`self.Cube`) true)
  (`PrimitiveComponent.SetMaterial` (`self.Cube`) 0 "/Game/Materials/MI_PlatformFalling.MI_PlatformFalling")
  (`KismetSystemLibrary.Delay` 3.0)
  (`self.Reset`))

(event `Reset`
  ;[0.6083 0.6545 1] Reset Platform
  (`KismetSystemLibrary.PrintString` "Resetting!" true true (struct :`R` 0.501961 :`G` 0.478431 :`B` 1.0 :`A` 1.0))
  (set `self.Reset Transform` (`SceneComponent.K2_GetComponentToWorld` (`self.Cube`)))
  (`PrimitiveComponent.SetSimulatePhysics` (`self.Cube`) false)
  (`PrimitiveComponent.SetMaterial` (`self.Cube`) 0 "/Game/Materials/MI_PlatformResetting.MI_PlatformResetting")
  (bind (_direction _newtrack_0) (`Timeline|Go Back To Start` :!via `PlayFromStart`)
    (:`Update`
      (bind (_returnvalue_location _returnvalue_rotation) (`KismetMathLibrary.BreakTransform` (`KismetMathLibrary.TLerp` (`self.Reset Transform`) (`self.Starting Transform`) _newtrack_0)))
      (`SceneComponent.K2_SetWorldLocationAndRotation` (`self.Cube`) _returnvalue_location _returnvalue_rotation false false))
    (:`Finished`
      (set `self.Ready` true)
      (`PrimitiveComponent.SetMaterial` (`self.Cube`) 0 "/Game/Materials/MI_PlatformReady.MI_PlatformReady"))))

(fn `UserConstructionScript`)