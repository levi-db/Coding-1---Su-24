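; Demo actor for loops and arrays, printing results to screen from looping events and key presses.
; BeginPlay starts a delayed game loop and a self-calling counter loop, while keys trigger a while loop and name-array tests.
; A self-calling event recolors a BP_Key via dynamic material every half second.
; Its reset check is always true, so both arrays reshuffle on every pass.
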(event `self.ReceiveBeginPlay`
  (`KismetSystemLibrary.PrintString` "Loops and Lists is running :)")
  (`|ExecutionSequence`
    (:`then_0`
      ;[1 1 1] Setup for Loops
      (`self.Simple Game Loop`)
      (`self.EnableInput` (`GameplayStatics.GetPlayerController` 0))
      (`self.Recursive Loop`))
    (:`then_1`
      ;[0.2778 0.2778 0.2778] Setup for Lists
      (bind _outactors (`GameplayStatics.GetAllActorsOfClass` "/Game/BluePrints/BP_Key.BP_Key_C"))
      (set `self.Keys` _outactors)
      (`self.Change Key Color`))))

(event `Simple Game Loop`
  (`KismetSystemLibrary.PrintString` "Starting Game Loop" true true (struct :`R` 0.015518 :`B` 1.0 :`A` 1.0) 0.6 :!label _label)
  (`KismetSystemLibrary.Delay` 1.0)
  (goto _label))

(event `self.ReceiveTick`
  (params (DeltaSeconds :type "Float (single-precision)")))

(event `InputAction|Start While Loop`
  (params (Key :type "Key Structure"))
  (bind _while_loop_counter (`self.While Loop Counter`))
  (:`Pressed`
    (`KismetSystemLibrary.PrintString` "Starting While Loop :)")
    (while (< (`self.While Loop Counter`) 25)
      ;[0.5782 0.5986 1] The While Loop's Body
      (`/Engine/EditorBlueprintResources/StandardMacros.IncrementInt` _while_loop_counter
        (:`  `
          (`KismetSystemLibrary.PrintString` (`KismetStringLibrary.Concat_StrStr` "This While Loop has run " (`KismetStringLibrary.Conv_IntToString` _while_loop_counter) " times.") true true (`KismetMathLibrary.MakeColor` (`KismetMathLibrary.RandomFloat`) (`KismetMathLibrary.RandomFloat`) (`KismetMathLibrary.RandomFloat`))))))
    (`KismetSystemLibrary.PrintString` "The While Loop is complete!")
    (set `self.While Loop Counter` 0)))

(event `Recursive Loop`
  (bind _recursion_counter (`self.Recursion Counter`))
  ;[0.7177 1 0.6659] Recursive Loop
  (if (< (`self.Recursion Counter`) 5)
    (`/Engine/EditorBlueprintResources/StandardMacros.IncrementInt` _recursion_counter
      (:`  `
        (`KismetSystemLibrary.PrintString` (`KismetStringLibrary.Concat_StrStr` "The Recursive Loop has run " (`KismetStringLibrary.Conv_IntToString` _recursion_counter) " times.") true true (struct :`R` 1.0 :`G` 0.342392 :`B` 0.442285 :`A` 1.0) 1.2)
        (`KismetSystemLibrary.Delay` 4.0)))
    (else
      (`KismetSystemLibrary.PrintString` "Resetting Recursive Loop :)")
      (set `self.Recursion Counter` 0)))
  (`self.Recursive Loop`) ; Loop calls itself
)

(event `Key|Six`
  (params (Key :type "Key Structure"))
  (:`Pressed`
    (`self.First Array Test`)))

(event `First Array Test`
  (bind _array (`|MakeArray` "Leia" "Luke" "Han" "Chewie" "Artoo" "Threepeeoh"))
  (`KismetSystemLibrary.PrintString` (`KismetStringLibrary.Concat_StrStr` "Our array of names has " (`KismetStringLibrary.Conv_IntToString` (`KismetArrayLibrary.Array_Length` _array)) " names in it."))
  (`KismetSystemLibrary.PrintString` (`KismetStringLibrary.Concat_StrStr` "The first name is our array is " (`|GetArrayItem` _array) ".")))

(event `Key|Five`
  (params (Key :type "Key Structure"))
  (:`Pressed`
    (`self.List All Names`)))

(event `List All Names`
  (for (_array_element _array_index) (`|MakeArray` "Leia" "Luke" "Han" "Chewie" "Artoo" "Threepeeoh")
    (`KismetSystemLibrary.PrintString` (`KismetStringLibrary.Concat_StrStr` (`KismetStringLibrary.Conv_IntToString` (+ _array_index 1)) ". " _array_element))))

(event `Change Key Color`
  (bind _keys (`self.Keys`))
  (bind _output (`|GetArrayItem` _keys (`self.Color Key Index`)))
  (if (or (>= (`self.Color Key Index`) (`KismetArrayLibrary.Array_Length` (`self.Colors`))) (<= (`self.Color Key Index`) (`KismetArrayLibrary.Array_Length` (`self.Colors`))))
    ;[1 0.584 0.4906] Shuffle & Reset
    (`KismetArrayLibrary.Array_Shuffle` (`self.Colors`))
    (`KismetArrayLibrary.Array_Shuffle` _keys)
    (set `self.Color Key Index` 0))
  (`/Engine/EditorBlueprintResources/StandardMacros.IsValid` _output
    (:`Is Valid`
      ;[0.9 1 0.6663] Setting Color of Key
      (bind _returnvalue (`PrimitiveComponent.CreateDynamicMaterialInstance` (`/Game/BluePrints/BP_Key.Cylinder` _output) 0 "/Game/Materials/M_Base.M_Base" "None"))
      (`MaterialInstanceDynamic.SetVectorParameterValue` _returnvalue "Base Color" (`KismetMathLibrary.Conv_ColorToLinearColor` (`|GetArrayItem` (`self.Colors`) (`self.Color Key Index`)))))
    (:`Is Not Valid`
      (bind _outactors (`GameplayStatics.GetAllActorsOfClass` "/Game/BluePrints/BP_Key.BP_Key_C")) ; If a key is missing, look at all keys and reset the lists of keys.
      (set `self.Keys` _outactors)))
  (`/Engine/EditorBlueprintResources/StandardMacros.IncrementInt` (`self.Color Key Index`)
    (:`  `
      (`KismetSystemLibrary.Delay` 0.5)
      (`self.Change Key Color`) ; Start the loop over again
    )))

(fn `UserConstructionScript`)