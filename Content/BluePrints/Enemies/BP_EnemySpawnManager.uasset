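; Enemy spawn manager actor that runs endless waves of BP_Enemy at placed spawner locations.
; On BeginPlay it gathers every BP_EnemySpawner and spawns one enemy at each, handing it a manager reference and counting it.
; RemoveEnemy&Check decrements that count and, when none remain, starts the next wave after a short delay.
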(event `self.ReceiveBeginPlay`
  (`KismetSystemLibrary.PrintString` "Enemy spawn manager is Ready" true true (struct :`R` 0.402778 :`G` 0.046339 :`A` 1.0))
  (bind _outactors (`GameplayStatics.GetAllActorsOfClass` "/Game/BluePrints/Enemies/BP_EnemySpawner.BP_EnemySpawner_C"))
  (set `self.Spawners` _outactors)
  (`self.Spawn Enemies`))

(event `Spawn Enemies`
  (for _array_element (`self.Spawners`)
    (bind (_returnvalue_location _returnvalue_rotation) (`KismetMathLibrary.BreakTransform` (`SceneComponent.K2_GetComponentToWorld` (`/Game/BluePrints/Enemies/BP_EnemySpawner.DefaultSceneRoot` _array_element))))
    (bind _returnvalue (`|SpawnActorFromClass` "/Game/BluePrints/Enemies/BP_Enemy.BP_Enemy_C" (`KismetMathLibrary.MakeTransform` _returnvalue_location _returnvalue_rotation) "Undefined" "MultiplyWithRoot" null null))
    (set `/Game/BluePrints/Enemies/BP_Enemy.Manager` self _returnvalue)
    (`/Engine/EditorBlueprintResources/StandardMacros.IncrementInt` (`self.Current Enemy Total`))))

(event `Remove Enemy & Check`
  (`/Engine/EditorBlueprintResources/StandardMacros.DecrementInt` (`self.Current Enemy Total`)
    (:`  `
      (if (not (> (`self.Current Enemy Total`) 0))
        (`KismetSystemLibrary.PrintString` "New wave incoming!!!!" true true (struct :`R` 0.427083 :`G` 0.002525 :`A` 1.0) 5.0)
        (`KismetSystemLibrary.Delay` 5.0)
        (`self.Spawn Enemies`)))))

(fn `UserConstructionScript`)